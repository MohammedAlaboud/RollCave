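; Player Blueprint that moves a physics-driven static mesh and restarts the level when the player takes damage, such as from falling off.
; Movement axis inputs apply torque to the mesh as acceleration, scaled by a force multiplier.
; BeginPlay fades the camera in from black.
; AnyDamage passes through a DoOnce so only the first hit fades the camera out, waits, then reopens the current level by name.
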(event `self.ReceiveBeginPlay`
  ;[1 1 1] Fade in from black screen when starting the game
  (`PlayerCameraManager.StartCameraFade` :`self` (`GameplayStatics.GetPlayerCameraManager` 0) :`FromAlpha` 1.0 :`Duration` 2.0) ; Fade in when starting to play
)

(event `InputAxis|MoveForward&Backward`
  (params (AxisValue :type "Float (single-precision)"))
  ;[1 1 1] Input Processing
  (`PrimitiveComponent.AddTorqueInRadians` (`self.StaticMesh`) (`KismetMathLibrary.MakeVector` 0.0 (* AxisValue (`self.ForceMultiplier`))) "None" true))

(event `InputAxis|MoveRight&Left`
  (params (AxisValue :type "Float (single-precision)"))
  ;[1 1 1] Input Processing
  (`PrimitiveComponent.AddTorqueInRadians` (`self.StaticMesh`) (`KismetMathLibrary.MakeVector` (* AxisValue (`self.ForceMultiplier`))) "None" true))

(event `self.ReceiveAnyDamage`
  (params (Damage :type "Float (single-precision)") (DamageType :type "DamageType Object Reference") (InstigatedBy :type "Controller Object Reference") (DamageCauser :type "Actor Object Reference"))
  (`/Engine/EditorBlueprintResources/StandardMacros.DoOnce` false ; Want player do be damaged once before\nthe view fading out of the level and restarting\nthe game (to avoid fading out more than once \nduring gameplay)
    (:`Completed`
      ;[1 1 1] Fade to black and restart level
      (`PlayerCameraManager.StartCameraFade` (`GameplayStatics.GetPlayerCameraManager` 0) 0.0 1.0 0.5 (struct :`R` 0.0059 :`A` 1.0) false true) ; Fade out when falling off level
      (`KismetSystemLibrary.Delay` 0.5)
      (bind _returnvalue (`GameplayStatics.GetCurrentLevelName` true))
      (`GameplayStatics.OpenLevel` (`KismetStringLibrary.Conv_StringToName` _returnvalue)) ; input is case sensitive,\n so it converts it
    )))

(fn `UserConstructionScript`)